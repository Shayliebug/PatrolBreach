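; Guard pawn that investigates camera alerts, patrols the supplied points, then returns to where it started.
; InvestigateCameraAlert stores the patrol points, moves to the alert destination with AIMoveTo, then starts Patrol after a retriggerable delay whether or not the move succeeds.
; Patrol loops through the points with pauses, using a Patrolling flag that a new alert clears to break the loop.
; BeginPlay records the home location; the ReturnToGuardStation function is an empty stub.
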(event Custom|InvestigateCameraAlert
  (params (Destination :type Vector) (PatrolPoints :type Array%20of%20Actor%20Object%20References))
  (Development|PrintString "looking for player")
  (Variables|Default|SetPatrolling false)
  (Variables|Default|SetPatrolPoints PatrolPoints)
  (bind _movementresult (AI|AIMoveTo self Destination 0 (Variables|Default|GetAcceptance%20Radius) false)
    (:OnSuccess
      _)
    (:OnFail
      _))
  (switch Utilities|FlowControl|Switch|SwitchonEPathFollowingResult _movementresult
    (:Success
      _)
    (:Blocked
      _)
    (:OffPath
      _)
    (:Invalid
      _))
  (Utilities|FlowControl|RetriggerableDelay 2.0)
  (CallFunction|Patrol))

(event Custom|Patrol
  (Variables|Default|SetIndex 0) ; reset patrol index.
  (Variables|Default|SetPatrolling true)
  (Development|PrintString "now patrolling")
  (AI|AIMoveTo self (Transformation|GetActorLocation (Utilities|Array|Get(acopy) (Variables|Default|GetPatrolPoints) (Variables|Default|GetIndex))) 0 (Variables|Default|GetAcceptance%20Radius) false :!label _label
    (:OnSuccess
      _)
    (:OnFail
      _))
  (Utilities|FlowControl|Delay 2.0)
  (Math|Integer|IncrementInt (Variables|Default|GetIndex)
    (:%20%20
      (if (>= (Variables|Default|GetIndex) (Utilities|Array|Length (Variables|Default|GetPatrolPoints)))
        (Variables|Default|SetPatrolling false)
        (CallFunction|ReturntoStation)
        (elif (Variables|Default|GetPatrolling)
          (goto _label)
          (else
            (Development|PrintString "actively seeking the player now, cancelling patrol")))))))

(event Custom|Return%20to%20Station
  (AI|AIMoveTo self (Variables|Default|GetStartLocation) 0 (Variables|Default|GetAcceptance%20Radius) false))

(event EventBeginPlay
  (Variables|Default|SetStartLocation (Transformation|GetWorldLocation (Variables|Collision|GetCapsuleComponent))))

(fn ConstructionScript)

(fn ReturntoGuardStation)